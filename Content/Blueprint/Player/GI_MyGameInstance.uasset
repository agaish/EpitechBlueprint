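; Game instance Blueprint that saves the player's high score to a save slot.
; Its Savescore event loads the existing SG_SavedScore, or creates one seeded with the new score, then writes it back to the slot.
; For an existing save, the high score is set from CompareNewScore, whose graph holds a larger-value SelectInt that appears unconnected.
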(event `Save score`
  (params (`New score` :type Integer))
  (set `self.New Score` `New score`)
  (bind _returnvalue (`GameplayStatics.DoesSaveGameExist` (`self.Save name`)))
  (if _returnvalue
    (bind _returnvalue_2 (`GameplayStatics.LoadGameFromSlot` (`self.Save name`)))
    (bind _assg_saved_score (cast `/Game/Blueprint/Player/SG_SavedScore` _returnvalue_2))
    (bind _output_get (set `self.Save REF` _assg_saved_score))
    (set `/Game/Blueprint/Player/SG_SavedScore.Highscore` (`self.Compare new score` (`self.New Score`) (`/Game/Blueprint/Player/SG_SavedScore.Highscore` _output_get)) _output_get)
    (else
      (bind _returnvalue_3 (`GameplayStatics.CreateSaveGameObject` "/Game/Blueprint/Player/SG_SavedScore.SG_SavedScore_C"))
      (bind _output_get_2 (set `self.Save REF` _returnvalue_3))
      (bind _assg_saved_score_2 (cast `/Game/Blueprint/Player/SG_SavedScore` _output_get_2))
      (set `/Game/Blueprint/Player/SG_SavedScore.Highscore` (`self.New Score`) _assg_saved_score_2)))
  (`GameplayStatics.SaveGameToSlot` (`self.Save REF`) (`self.Save name`)))