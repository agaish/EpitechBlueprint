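; BP_FakePlateform is an obstacle with two platforms, one randomly chosen as the fake that falls.
; BeginPlay runs the parent setup, stores the second platform's transform, rolls IsLeftFake and calls SwitchColor on that second platform.
; When the player character overlaps either trigger box, shared logic calls Fall on the fake platform with its saved transform, whichever box was touched.
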(event `self.ReceiveBeginPlay`
  ;[0 1 0.0356] Begin play + set 2nd transform and color
  (`parent.ReceiveBeginPlay`)
  (set `self.InitialTransform2` (`SceneComponent.K2_GetComponentToWorld` (`self.Plateform2`)))
  (set `self.IsLeftFake?` (`KismetMathLibrary.RandomBool`))
  (`self.SwitchColor` (`self.Plateform2`)))

(event `self.Box2.OnComponentBeginOverlap`
  (params (OverlappedComponent :type "PrimitiveComponent Object Reference") (OtherActor :type "Actor Object Reference") (OtherComp :type "PrimitiveComponent Object Reference") (OtherBodyIndex :type Integer) (bFromSweep :type Boolean) (SweepResult :type "HitResult Structure (by ref)"))
  (bind _plateform (`self.Plateform`))
  (bind _plateform2 (`self.Plateform2`))
  ;[0 1 0.0356] Actor collision check + which plateform should fall
  (if (== OtherActor (`GameplayStatics.GetPlayerCharacter` 0))
    (if (`self.IsLeftFake?`) :!label _label
      ;[0 1 0.0356] Plateform fall
      (`/Engine/EditorBlueprintResources/StandardMacros.IsValid` _plateform
        (:`Is Valid`
          (`self.Fall` _plateform (`self.Initial transform`))))
      (else
        (`/Engine/EditorBlueprintResources/StandardMacros.IsValid` _plateform2
          (:`Is Valid`
            (`self.Fall` _plateform2 (`self.InitialTransform2`))))))))

(event `self.Box.OnComponentBeginOverlap`
  (params (OverlappedComponent :type "PrimitiveComponent Object Reference") (OtherActor :type "Actor Object Reference") (OtherComp :type "PrimitiveComponent Object Reference") (OtherBodyIndex :type Integer) (bFromSweep :type Boolean) (SweepResult :type "HitResult Structure (by ref)"))
  ;[0 1 0.0356] Actor collision check + which plateform should fall
  (if (== OtherActor (`GameplayStatics.GetPlayerCharacter` 0))
    (goto _label)))

(fn `UserConstructionScript`
  (`parent.UserConstructionScript`))