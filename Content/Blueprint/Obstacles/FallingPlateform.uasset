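; Falling platform obstacle that drops after the player character steps into its trigger box.
; On begin play it caches the platform's transform and assigns a random red, green or blue material.
; Overlap on a Falling-type platform waits a configurable delay, then enables physics simulation on it.
; Three seconds later it either stops physics and teleports back to its start or destroys the platform component, depending on a respawn flag.
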(event `self.ReceiveBeginPlay`
  (set `self.Initial transform` (`SceneComponent.K2_GetComponentToWorld` (`self.Plateform`)))
  (`self.SwitchColor` (`self.Plateform`)))

(event `Fall`
  (params (Target :type "PrimitiveComponent Object Reference"))
  (`KismetSystemLibrary.Delay` (`self.Duration before falling`))
  (`PrimitiveComponent.SetSimulatePhysics` Target true)
  (`KismetSystemLibrary.Delay` 3.0)
  (if (`self.bShouldRespawn?`)
    (`PrimitiveComponent.SetSimulatePhysics` (`self.Plateform`) false)
    (`PrimitiveComponent.SetSimulatePhysics` Target false)
    (`SceneComponent.K2_SetWorldTransform` (`self.Plateform`) (`self.Initial transform`) false true)
    (else
      (`ActorComponent.K2_DestroyComponent` Target))))

(event `self.Box.OnComponentBeginOverlap`
  (params (OverlappedComponent :type "PrimitiveComponent Object Reference") (OtherActor :type "Actor Object Reference") (OtherComp :type "PrimitiveComponent Object Reference") (OtherBodyIndex :type Integer) (bFromSweep :type Boolean) (SweepResult :type "HitResult Structure (by ref)"))
  (if (== OtherActor (`GameplayStatics.GetPlayerCharacter` 0))
    (switch `/Game/Blueprint/Obstacles/E_PlateformType` (`self.PlateformType`)
      (:`NewEnumerator0`
        (`self.Fall` (`self.Plateform`))))))

(fn `SwitchColor`
  (params (Target :type "PrimitiveComponent Object Reference"))
  (`PrimitiveComponent.SetMaterial` Target 0 (select `int` (`KismetMathLibrary.RandomIntegerInRange` 0 2) :`0` "/Game/Material/MI_Red.MI_Red" :`1` "/Game/Material/MI_Green.MI_Green" :`2` "/Game/Material/MI_Blue.MI_Blue" :!type "MaterialInterface Object Reference")))

(fn `UserConstructionScript`)